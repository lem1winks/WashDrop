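; Main actor for a falling game: the player drops past a building, steering with A/D to collect Dirt for multiplied score and avoid Balconies.
; Tick runs the flag-driven sequence from camera intro and lift click to splat and retry button.
; The fall is faked by looping building panels, each wrap spawning random objects that Tick moves upward.
; Streaks raise the wrap limit, lengthening the fall until the ground scrolls in.
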(event OnClicked(Test)
  (params (TouchedComponent :type Primitive%20Component%20Object%20Reference))
  ;[1 1 1] Lift Button Clicked
  (Rendering|ToggleVisibility (stale OnInputTouchBegin(Test) TouchedComponent) false)
  (Variables|Default|SetLiftClicked true)
  ;[1 1 1] Scream Sound
  (Audio|Components|Audio|Play (Variables|Default|GetAudio_Scream) 0.0))

(event OnComponentBeginOverlap(Box1)
  (params (OtherActor :type Actor%20Object%20Reference) (OtherComp :type Primitive%20Component%20Object%20Reference) (OtherBodyIndex :type Integer))
  (bind _box1 (Variables|Default|GetBox1))
  (bind _playermain (Variables|Default|GetPlayerMain))
  ;[1 1 1] when collide with dirt and balcony
  (if (== (Utilities|GetClass OtherActor) "/Game/Blueprints/Balcony.Balcony_C")
    ;[1 1 1] Damages player
    (Variables|Default|SetScore (- (Variables|Default|GetScore) 1))
    (Variables|Default|SetMultiplier 0)
    ;[1 1 1] flash when hit
    (Collision|SetCollisionEnabled _box1 "NoCollision")
    (Rendering|Material|SetMaterial _playermain 0 "/Game/Textures/Character_Mat2.Character_Mat2")
    (Utilities|FlowControl|Delay 0.1)
    (Rendering|Material|SetMaterial _playermain 0 "/Game/Textures/Character_Mat.Character_Mat")
    (Utilities|FlowControl|Delay 0.1)
    (Collision|SetCollisionEnabled _box1 "QueryAndPhysics")
    (else
      (Actor|DestroyActor OtherActor)
      ;[1 1 1] Multiplier for score
      (Variables|Default|SetMultiplier (+ (Variables|Default|GetMultiplier) 1))
      (Variables|Default|SetScore (+ (Variables|Default|GetScore) (* (Variables|Default|GetBaseScore) (Variables|Default|GetMultiplier))))
      ;[1 1 1] Sets score to 0 if minus
      (if (< (Variables|Default|GetScore) 0)
        (Variables|Default|SetScore 0))
      (if (Variables|Default|GetSpawnNewLayers)
        (if (== (Variables|Default|GetMultiplier) 3)
          (Variables|Default|SetSpawnTotal (+ 1 (Variables|Default|GetSpawnTotal)))
          (elif (== (Variables|Default|GetMultiplier) 6)
            (Variables|Default|SetSpawnTotal (+ (Variables|Default|GetSpawnTotal) 3))
            (elif (>= (Variables|Default|GetMultiplier) 9)
              (Variables|Default|SetSpawnTotal (+ (Variables|Default|GetSpawnTotal) 5)))))))))

(event OnClicked(TryAgainButton)
  (params (TouchedComponent :type Primitive%20Component%20Object%20Reference))
  ;[1 1 1] Try Again Button
  (Game|OpenLevel(byName) "Test_FallingLevel"))

(event OnInputTouchBegin(PlayButton)
  (params (FingerIndex :type ETouchIndex%20Enum) (TouchedComponent :type Primitive%20Component%20Object%20Reference))
  ;[1 1 1] Play Button Clicked
  (Variables|Default|SetShouldStart true))

(event OnInputTouchBegin(Test)
  (params (FingerIndex :type ETouchIndex%20Enum) (TouchedComponent :type Primitive%20Component%20Object%20Reference))
  ;[1 1 1] Lift Button Clicked
  (Rendering|ToggleVisibility TouchedComponent false)
  (Variables|Default|SetLiftClicked true)
  ;[1 1 1] Scream Sound
  (Audio|Components|Audio|Play (Variables|Default|GetAudio_Scream) 0.0))

(event OnClicked(PlayButton)
  (params (TouchedComponent :type Primitive%20Component%20Object%20Reference))
  ;[1 1 1] Play Button Clicked
  (Variables|Default|SetShouldStart true))

(event OnInputTouchBegin(TryAgainButton)
  (params (FingerIndex :type ETouchIndex%20Enum) (TouchedComponent :type Primitive%20Component%20Object%20Reference))
  ;[1 1 1] Try Again Button
  (Game|OpenLevel(byName) "Test_FallingLevel"))

(event EventTick
  (params (DeltaSeconds :type Float%20%28single-precision%29))
  (bind _bottom (Variables|Default|GetBottom))
  (bind _tryagainbutton (Variables|Default|GetTryAgainButton))
  (bind _camera (Variables|Default|GetCamera))
  (bind _playermain (Variables|Default|GetPlayerMain))
  (bind _playermain_2 (Variables|Default|GetPlayerMain))
  ;[1 1 1] Sets Camera
  (Game|Player|SetViewTargetwithBlend (Game|GetPlayerController 0) self 0.0 "VTBlend_Linear" 0.0 false)
  (CallFunction|Menu)
  (Input|EnableInput (Game|GetPlayerController 0))
  ;[1 1 1] If started from the menu, starts camera moving
  (if (Variables|Default|GetStartGame)
    (if (Variables|Default|GetShouldStart)
      (if (Variables|Default|GetShouldStartLOCK)
        ;[1 1 1] Checks If camera is in start/ready position
        (Transformation|AddRelativeLocation _camera "-10.000000, 0, 0" false)
        (if (<= (.X (Math|Vector|BreakVector (Variables|/Script/Engine.SceneComponent|GetRelativeLocation _camera))) -6.6e+02)
          (Variables|Default|SetShouldStartLOCK false)
          (if (Variables|Default|GetLiftClicked) :!label _label
            (if (Variables|Default|GetInPosition)
              ;[1 1 1] Control Actions
              (if (Variables|Default|GetLeftHeldDown)
                (if (<= (.Y (Math|Vector|BreakVector (Variables|/Script/Engine.SceneComponent|GetRelativeLocation _playermain))) -1.7e+02)
                  _
                  (else
                    (Transformation|AddRelativeLocation _playermain "0.000000,-10.000000, 0" false)
                    (if (Variables|Default|GetRightHeldDown) :!label _label_2
                      (if (>= (.Y (Math|Vector|BreakVector (Variables|/Script/Engine.SceneComponent|GetRelativeLocation _playermain))) 1.7e+02)
                        _
                        (else
                          (Transformation|AddRelativeLocation _playermain "0.000000,10.000000, 0" false))))))
                (else
                  (goto _label_2)))
              (CallFunction|PanBuidling)
              (if (Variables|Default|GetMoveResetButton)
                ;[1 1 1] Moves Reset Button into Position
                (if (<= (.X (Math|Vector|BreakVector (Variables|/Script/Engine.SceneComponent|GetRelativeLocation _tryagainbutton))) -2e+01)
                  (Variables|Default|SetMoveResetButton false)
                  (else
                    (Transformation|AddRelativeLocation _tryagainbutton "-10.000000,0.000000,0.000000" false)))
                (elif (Variables|Default|GetPlaySplat)
                  ;[1 1 1] Play Splat
                  (Rendering|Material|SetMaterial _bottom 0 "/Game/Materials/bacbuildBottomSmlBlood_Mat.bacbuildBottomSmlBlood_Mat")
                  (Utilities|FlowControl|Delay 0.05)
                  (Rendering|Material|SetMaterial _bottom 0 "/Game/Materials/bacbuildBottomBlood_Mat.bacbuildBottomBlood_Mat")
                  (Variables|Default|SetPlaySplat false)
                  ;[1 1 1] Play Splat Sound
                  (Audio|Components|Audio|SetSound (Variables|Default|GetAudio_Scream) "/Game/Audio/47982__benhillyard__vocal-splat-10.47982__benhillyard__vocal-splat-10")
                  (Utilities|FlowControl|Delay 0.5)
                  (Variables|Default|SetMoveResetButton true)
                  (else
                    ;[1 1 1] Move spawned windows upwards
                    (for _array_element (Variables|Default|GetDirtPickups)
                      (Class|Actor|AddActorLocalTransform _array_element (Math|Conversions|ToTransform(Vector) "0, 0,10.000000") false)
                      (if (> (.Z (Math|Vector|BreakVector (Transformation|GetActorLocation _array_element))) 9e+02)
                        (Actor|DestroyActor _array_element)
                        (Utilities|Array|RemoveItem (Variables|Default|GetDirtPickups) _array_element))))))
              (else
                ;[1 1 1] When lift is clicked, player falls into Position
                (Transformation|AddRelativeLocation _playermain_2 "-10.000000,0.000000,0.000000" false)
                (if (<= (.X (Math|Vector|BreakVector (Variables|/Script/Engine.SceneComponent|GetRelativeLocation _playermain_2))) -6.3e+02)
                  (Variables|Default|SetInPosition true))))))
        (else
          (goto _label))))))

(event EventBeginPlay
  ;[1 1 1] Sets Resolution
  (Development|ExecuteConsoleCommand "setres 640x960 "))

(event Input|KeyboardEvents|A
  ;[1 1 1] Mapping Controls
  (:Pressed
    (Variables|Default|SetLeftHeldDown true))
  (:Released
    (Variables|Default|SetLeftHeldDown false)))

(event Input|KeyboardEvents|D
  ;[1 1 1] Mapping Controls
  (:Pressed
    (Variables|Default|SetRightHeldDown true))
  (:Released
    (Variables|Default|SetRightHeldDown false)))

(fn ConstructionScript
  (bind _buildingarray (Variables|Default|GetBuildingArray))
  ;[1 1 1] Adds Scrolling Background to Array
  (Utilities|Array|Add _buildingarray (Variables|Default|GetBuilding04))
  (Utilities|Array|Add _buildingarray (Variables|Default|GetBuilding01))
  (Utilities|Array|Add _buildingarray (Variables|Default|GetBuilding02))
  (Utilities|Array|Add _buildingarray (Variables|Default|GetBuilding03))
  ;[1 1 1] Gets Spawn Locations
  (Variables|Default|SetSpawnLoc01 (Math|Conversions|ToTransform(Vector) (Transformation|GetWorldLocation (Variables|Default|GetSpawnPoint01))))
  (Variables|Default|SetSpawnLoc02 (Math|Conversions|ToTransform(Vector) (Transformation|GetWorldLocation (Variables|Default|GetSpawnPoint02))))
  (Variables|Default|SetSpawnLoc03 (Math|Conversions|ToTransform(Vector) (Transformation|GetWorldLocation (Variables|Default|GetSpawnPoint03))))
  (Variables|Default|SetSpawnLoc04 (Math|Conversions|ToTransform(Vector) (Transformation|GetWorldLocation (Variables|Default|GetSpawnPoint04))))
  (Variables|Default|SetSpawnLoc05 (Math|Conversions|ToTransform(Vector) (Transformation|GetWorldLocation (Variables|Default|GetSpawnPoint05))))
  (Variables|Default|SetSpawnLoc06 (Math|Conversions|ToTransform(Vector) (Transformation|GetWorldLocation (Variables|Default|GetSpawnPoint06))))
  (Variables|Default|SetSpawnLoc07 (Math|Conversions|ToTransform(Vector) (Transformation|GetWorldLocation (Variables|Default|GetSpawnPoint07))))
  (Variables|Default|SetSpawnLoc08 (Math|Conversions|ToTransform(Vector) (Transformation|GetWorldLocation (Variables|Default|GetSpawnPoint08)))))

(fn PanBuidling
  (bind _returnvalue (Math|Vector|MakeVector 1e+01 0.0 0.0))
  (bind _playermain (Variables|Default|GetPlayerMain))
  (bind _bottom (Variables|Default|GetBottom))
  ;[1 1 1] Checks spawncount before spawn
  (if (>= (Variables|Default|GetSpawnCount) (Variables|Default|GetSpawnTotal))
    (Variables|Default|SetSpawnNewLayers false)
    ;[1 1 1] Moves the BottomFloor up into Position
    (if (>= (.X (Math|Vector|BreakVector (Variables|/Script/Engine.SceneComponent|GetRelativeLocation _bottom))) -7.5e+02)
      (if (Variables|Default|GetInEndPosition)
        ;[1 1 1] Toggle Score when player hits floor
        (if (Variables|Default|GetShowScore) :!label _label
          (Rendering|ToggleVisibility (Variables|Default|GetScoreText) false)
          (Variables|Default|SetShowScore false))
        (else
          ;[1 1 1] Stops at the bottom and dissapears
          (Transformation|AddRelativeLocation _playermain "-10.000000,0.000000,0.000000" false)
          (if (<= (.X (Math|Vector|BreakVector (Variables|/Script/Engine.SceneComponent|GetRelativeLocation _playermain))) -8e+02)
            (Rendering|ToggleVisibility _playermain false)
            (Variables|Default|SetInEndPosition true)
            (Variables|Default|SetPlaySplat true)
            (goto _label))))
      (else
        (for _array_element (Variables|Default|GetBuildingArray)
          (Transformation|AddRelativeLocation _array_element _returnvalue false))
        (Transformation|AddRelativeLocation _bottom _returnvalue false)))
    (else
      ;[1 1 1] Pans the backgorundimages resetting them when they are out of view
      (for _array_element_2 (Variables|Default|GetBuildingArray)
        (if (>= (.X (Math|Vector|BreakVector (Variables|/Script/Engine.SceneComponent|GetRelativeLocation _array_element_2))) 0.0)
          (Transformation|SetRelativeLocation _array_element_2 "-1500.000000, 0, 0" false)
          (CallFunction|SpawnObjects)
          ;[1 1 1] Adds 1 to the spawncount
          (Variables|Default|SetSpawnCount (+ (Variables|Default|GetSpawnCount) 1))
          (else
            (Transformation|AddRelativeLocation _array_element_2 _returnvalue false)))))))

(fn Menu
  (Variables|Default|SetStartGame true))

(fn SpawnObjects
  (bind _returnvalue (Math|Random|RandomBool))
  (bind _dirtpickups (Variables|Default|GetDirtPickups))
  ;[1 1 1] sets which spawns are active
  (Variables|Default|SetSpawn1 _returnvalue)
  (Variables|Default|SetSpawn2 _returnvalue)
  (Variables|Default|SetSpawn3 _returnvalue)
  (Variables|Default|SetSpawn4 _returnvalue)
  (Variables|Default|SetSpawn5 _returnvalue)
  (Variables|Default|SetSpawn6 _returnvalue)
  (Variables|Default|SetSpawn7 _returnvalue)
  (Variables|Default|SetSpawn8 _returnvalue)
  ;[1 1 1] Randomly picks dirt or balcony
  (if (Math|Random|RandomBool) :!label _label
    (Variables|Default|SetSpawnActor "/Game/Blueprints/Dirt.Dirt_C")
    (else
      (Variables|Default|SetSpawnActor "/Game/Blueprints/Balcony.Balcony_C")))
  ;[1 1 1] picks which spawn points activate
  (if (Variables|Default|GetSpawn1)
    (Variables|Default|SetSpawn1 false)
    ;[1 1 1] Spawns Actor at spawn points chosen
    (bind _returnvalue_2 (Game|SpawnActorfromClass (Variables|Default|GetSpawnActor) (Variables|Default|GetSpawnLoc05) true))
    ;[1 1 1] Adds Spawned Actors to Array
    (Utilities|Array|Add _dirtpickups _returnvalue_2)
    ;[1 1 1] Is Spawn Limit Reached?
    (Variables|Default|SetSpawnLimit (+ (Variables|Default|GetSpawnLimit) 1) :!label _label_2)
    (if (>= (Variables|Default|GetSpawnLimit) 8)
      (Variables|Default|SetSpawnLimit 0)
      (else
        (goto _label)))
    (elif (Variables|Default|GetSpawn2)
      (Variables|Default|SetSpawn2 false)
      (bind _returnvalue_3 (Game|SpawnActorfromClass (Variables|Default|GetSpawnActor) (Variables|Default|GetSpawnLoc06) true))
      (Utilities|Array|Add _dirtpickups _returnvalue_3)
      (goto _label_2)
      (elif (Variables|Default|GetSpawn3)
        (Variables|Default|SetSpawn3 false)
        (bind _returnvalue_4 (Game|SpawnActorfromClass (Variables|Default|GetSpawnActor) (Variables|Default|GetSpawnLoc07) true))
        (Utilities|Array|Add _dirtpickups _returnvalue_4)
        (goto _label_2)
        (elif (Variables|Default|GetSpawn4)
          (Variables|Default|SetSpawn4 false)
          (bind _returnvalue_5 (Game|SpawnActorfromClass (Variables|Default|GetSpawnActor) (Variables|Default|GetSpawnLoc08) true))
          (Utilities|Array|Add _dirtpickups _returnvalue_5)
          (goto _label_2)
          (elif (Variables|Default|GetSpawn5)
            (Variables|Default|SetSpawn5 false)
            (bind _returnvalue_6 (Game|SpawnActorfromClass (Variables|Default|GetSpawnActor) (Variables|Default|GetSpawnLoc01) true))
            (Utilities|Array|Add _dirtpickups _returnvalue_6)
            (goto _label_2)
            (elif (Variables|Default|GetSpawn6)
              (Variables|Default|SetSpawn6 false)
              (bind _returnvalue_7 (Game|SpawnActorfromClass (Variables|Default|GetSpawnActor) (Variables|Default|GetSpawnLoc02) true))
              (Utilities|Array|Add _dirtpickups _returnvalue_7)
              (goto _label_2)
              (elif (Variables|Default|GetSpawn7)
                (Variables|Default|SetSpawn7 false)
                (bind _returnvalue_8 (Game|SpawnActorfromClass (Variables|Default|GetSpawnActor) (Variables|Default|GetSpawnLoc03) true))
                (Utilities|Array|Add _dirtpickups _returnvalue_8)
                (goto _label_2)
                (elif (Variables|Default|GetSpawn8)
                  (Variables|Default|SetSpawn8 false)
                  (bind _returnvalue_9 (Game|SpawnActorfromClass (Variables|Default|GetSpawnActor) (Variables|Default|GetSpawnLoc04) true))
                  (Utilities|Array|Add _dirtpickups _returnvalue_9)
                  (goto _label_2))))))))))